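; Game mode that runs a seated audience: spawns it, sends it to seats and switches its action on the Exit state.
; On BeginPlay it caches the door, tagged audience spawn and seat rows, then after a short delay opens the door and spawns randomized audience humans in a grid.
; Each reserves a seat found by random retry, with no guard against all seats being taken.
; FindPlayerStart selects the PlayerStart tagged PlayerSpawn.
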(event Custom|SetCurrentState
  (params (CurrentState :type E_PresentationState%20Enum :default "NewEnumerator0"))
  ;[1 1 1] Set State
  (bind _output_get (Variables|Default|SetCurrentState CurrentState))
  (switch Utilities|FlowControl|Switch|SwitchonE_PresentationState _output_get
    (:NewEnumerator2
      (for _array_element (Variables|Default|GetAudience)
        (Default|SetCurrentAction _array_element "NewEnumerator3")))))

(event EventBeginPlay
  ;[1 1 1] Init
  (CallFunction|InitDefaults)
  (Utilities|FlowControl|Delay 3.0)
  ;[1 1 1] Audience Entrance
  (Default|SetDoorOpen (Variables|Default|GetBP_Door) true)
  (CallFunction|SpawnAudience))

(fn ConstructionScript)

(fn InitDefaults
  (Utilities|FlowControl|Sequence
    (:then_0
      ;[1 1 1] Door
      (bind _outactors (Actor|GetAllActorsOfClass "/Game/Blueprints/BP_Door.BP_Door_C"))
      (bind _output_get (Variables|Default|SetBP_Door (Utilities|Array|Get(acopy) _outactors)))
      ;[1 1 1] DEBUG
      (Utilities|FlowControl|Sequence
        (:then_0
          (if (not (Utilities|IsValid _output_get))
            (Development|PrintString "No Door implementing Interface_Door found!" true true "(R=1.000000,G=0.000000,B=0.000000,A=1.000000)" 1e+04)))))
    (:then_1
      ;[1 1 1] Audience Spawn
      (bind _outactors_2 (Actor|GetAllActorsOfClass "/Script/Engine.PlayerStart"))
      (for _array_element _outactors_2
        (if (Utilities|Name|Equal(Name) (Variables|/Script/Engine.PlayerStart|GetPlayerStartTag _array_element) "AudienceSpawn")
          (Variables|Default|SetAudienceSpawn _array_element)))
      (Utilities|IsValid (Variables|Default|GetAudienceSpawn)
        (:Is%20Not%20Valid
          (Development|PrintString "No PlayerStart with Tag \"AudienceSpawn\" found!" true true "(R=1.000000,G=0.000000,B=0.000000,A=1.000000)" 1e+04))))
    (:then_2
      ;[1 1 1] SeatRows
      (bind _outactors_3 (Actor|GetAllActorsOfClass "/Game/Blueprints/BP_SeatRows.BP_SeatRows_C"))
      (bind _output_get_2 (Variables|Default|SetSeatRows (Utilities|Array|Get(acopy) _outactors_3)))
      (Utilities|IsValid _output_get_2
        (:Is%20Not%20Valid
          (Development|PrintString "No BP_SeatRows found!" true true "(R=1.000000,G=0.000000,B=0.000000,A=1.000000)" 1e+04))))))

(fn SpawnAudience
  (bind _returnvalue (Class|KismetSystemLibrary|MakeLiteralInteger 20))
  (for _index (range 0 20)
    (bind _returnvalue_2 (Game|SpawnActorfromClass "/Game/Blueprints/Audience/BP_AudienceHuman.BP_AudienceHuman_C" (Math|Transform|MakeTransform (+ (Transformation|GetActorLocation (Variables|Default|GetAudienceSpawn)) (Math|Vector|MakeVector (* (/ _index _returnvalue) -1e+02) (* (Math|Integer|%(Integer) _index _returnvalue) 1e+02) 0.0)) "0, 0, 0" "1,1,1") "AdjustIfPossibleButAlwaysSpawn" 0 (Math|Random|RandomBool) (Math|Random|RandomBool) 0))
    (bind _seat (CallFunction|GetUnusedSeat))
    (Default|MovetoSeat _returnvalue_2 _seat true)
    (Utilities|Array|Add (Variables|Default|GetAudience) _returnvalue_2)))

(fn GetUnusedSeat
  (bind _seatrows (Variables|Default|GetSeatRows))
  (bind _rows (Variables|/Game/Blueprints/BP_SeatRows.BP_SeatRows_C|GetRows _seatrows))
  (if (LocalVariables|GetUsed) :!label _label
    (bind _output_get (LocalVariables|SetRow (Utilities|Array|Get(acopy) _rows (Math|Random|RandomInteger (Utilities|Array|Length _rows)))))
    (bind _output_get_2 (LocalVariables|SetRet (Utilities|Array|Get(acopy) (Variables|/Game/Blueprints/BP_SeatRow.BP_SeatRow_C|GetSeats _output_get) (Math|Random|RandomInteger (Utilities|Array|Length (Variables|/Game/Blueprints/BP_SeatRow.BP_SeatRow_C|GetSeats _output_get))))))
    (LocalVariables|SetUsed (Variables|/Game/Blueprints/BP_Seat.BP_Seat_C|GetReserverd _output_get_2))
    (goto _label)
    (else
      (Default|SetReserved (LocalVariables|GetRet) true)
      (return (LocalVariables|GetRet)))))

(fn FindPlayerStart
  (params (Player :type Controller%20Object%20Reference) (IncomingName :type String))
  (bind _outactors (Actor|GetAllActorsOfClass "/Script/Engine.PlayerStart"))
  (for _array_element _outactors
    (if (Utilities|Name|Equal(Name) (Variables|/Script/Engine.PlayerStart|GetPlayerStartTag _array_element) "PlayerSpawn")
      (return _array_element)))
  (return 0))