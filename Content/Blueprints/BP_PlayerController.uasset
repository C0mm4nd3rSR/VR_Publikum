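; Player controller that puts up the in-game HUD and provides a debug-style key for stepping through presentation states.
; On BeginPlay it creates the W_Ingame widget for itself and adds it to the viewport.
; Pressing H, marked as a presentation hack, advances the BP_Gamemode current presentation state by one, clamped at the third enum value.
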(event EventBeginPlay
  ;[1 1 1] Widget
  (bind _returnvalue (UserInterface|CreateWidget "/Game/Widgets/W_Ingame.W_Ingame_C" self))
  (UserInterface|Viewport|AddtoViewport _returnvalue 0))

(event Input|KeyboardEvents|H
  (params (Key :type Key%20Structure))
  ;[1 1 1] Presentation HACK
  (:Pressed
    (bind _asbp_gamemode (Utilities|Casting|CastToBP_Gamemode (Game|GetGameMode)))
    (Default|SetCurrentState _asbp_gamemode (Utilities|Enum|ByteToEnumE_PresentationState (Class|KismetMathLibrary|BMin (+ (Variables|/Game/Blueprints/BP_Gamemode.BP_Gamemode_C|GetCurrentState _asbp_gamemode) 1) 2)))))

(fn ConstructionScript)