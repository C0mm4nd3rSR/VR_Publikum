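; BP_SeatRows procedurally builds a block of seat rows from BP_SeatRow child actors.
; When AllowRefresh is on, the construction script adds NUMSEATROWS child actor components, each placed at a multiple of SPAWNOFFSET from the origin.
; Each spawned child actor is cast to BP_SeatRow and appended to the Rows array, which the script does not clear beforehand.
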(fn ConstructionScript
  (if (Variables|Default|GetAllowRefresh)
    (for _index (range 0 (- (Variables|Default|GetNUM_SEAT_ROWS) 1))
      (bind _returnvalue (AddComponent|AddChildActorComponent false (Math|Transform|MakeTransform (* (Variables|Default|GetSPAWN_OFFSET) _index) "0, 0, 0" "1,1,1")))
      (ChildActorComponent|SetChildActorClass _returnvalue "/Game/Blueprints/BP_SeatRow.BP_SeatRow_C")
      (bind _asbp_seat_row (Utilities|Casting|CastToBP_SeatRow (Variables|/Script/Engine.ChildActorComponent|GetChildActor _returnvalue)))
      (Utilities|Array|Add (Variables|Default|GetRows) _asbp_seat_row))))