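; Audience member character that walks to an assigned seat, sits, and later exits to its spawn point.
; On spawn it picks a random mesh, materials, colours and height from DT_Appearance, filtered by gender and reputability.
; Overlapping another member makes a seated one stand back without collision or gravity while the walker pauses, then sit again.
; While seated, it turns with the seat and randomly plays data-table-driven facial morph animations.
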(event OnComponentBeginOverlap(LetPassBox)
  (params (OverlappedComponent :type Primitive%20Component%20Object%20Reference) (OtherActor :type Actor%20Object%20Reference) (OtherComp :type Primitive%20Component%20Object%20Reference) (OtherBodyIndex :type Integer) (bFromSweep :type Boolean) (SweepResult :type Hit%20Result%20Structure%20%28by%20ref%29))
  ;[1 1 1] LetSomeoneThrough
  (bind _asbp_audience_human (Utilities|Casting|CastToBP_AudienceHuman OtherActor))
  (if (!= _asbp_audience_human self)
    (switch Utilities|FlowControl|Switch|SwitchonE_CurrentActions (Variables|Default|GetCurrentAction)
      (:NewEnumerator1
        (Variables|Default|SetCurrentAction "NewEnumerator2")
        (Default|SetOccupied (Variables|Default|GetTargetSeat) false)
        (CallFunction|DelayPathfingtoLetSomeoneStandUp _asbp_audience_human 1.0)
        (Collision|SetCollisionEnabled (Variables|Collision|GetCapsuleComponent) "NoCollision")
        (Variables|/Script/Engine.CharacterMovementComponent|SetGravityScale (Variables|Character|GetCharacterMovement) 0.0)
        (Utilities|Set|Add (Variables|Default|GetCurrentAudienceLetThrought) _asbp_audience_human)))))

(event OnComponentEndOverlap(LetPassBox)
  (params (OverlappedComponent :type Primitive%20Component%20Object%20Reference) (OtherActor :type Actor%20Object%20Reference) (OtherComp :type Primitive%20Component%20Object%20Reference) (OtherBodyIndex :type Integer))
  (bind _currentaudienceletthrought (Variables|Default|GetCurrentAudienceLetThrought))
  ;[1 1 1] LetSomeoneThrough
  (bind _asbp_audience_human (Utilities|Casting|CastToBP_AudienceHuman OtherActor))
  (if (!= (stale OnComponentBeginOverlap(LetPassBox) _asbp_audience_human) self)
    (switch Utilities|FlowControl|Switch|SwitchonE_CurrentActions (Variables|Default|GetCurrentAction)
      (:NewEnumerator2
        (Utilities|FlowControl|RetriggerableDelay 1.0)
        (Utilities|Set|Remove _currentaudienceletthrought _asbp_audience_human)
        (if (== (Utilities|Set|Length _currentaudienceletthrought) 0)
          (Variables|Default|SetCurrentAction "NewEnumerator1")
          (Default|SetOccupied (Variables|Default|GetTargetSeat) true)
          (Collision|SetCollisionEnabled (Variables|Collision|GetCapsuleComponent) "QueryAndPhysics")
          (Variables|/Script/Engine.CharacterMovementComponent|SetGravityScale (Variables|Character|GetCharacterMovement) 1.0))))))

(event Custom|MoveToSeat
  (params (TargetSeat :type BP%20Seat%20Object%20Reference) (InitalDelay :type Boolean))
  ;[1 1 1] Move To
  (Utilities|FlowControl|RetriggerableDelay (select InitalDelay (Math|Random|RandomFloatinRange 1.0 1e+01) 0.0))
  (Variables|Default|SetTargetSeat TargetSeat)
  (Pawn|SpawnDefaultController)
  (AI|AIMoveTo (AI|GetAIController self) self (Transformation|GetActorLocation (Variables|Default|GetTargetSeat)) 0 5.0 false
    (:OnSuccess
      (Variables|Default|SetCurrentAction "NewEnumerator1")
      (Default|SetOccupied (Variables|Default|GetTargetSeat) true)
      (AI|Navigation|StopMovement (Pawn|GetController)))))

(event Custom|SetCurrentAction
  (params (CurrentAction :type E_CurrentActions%20Enum :default "NewEnumerator0"))
  ;[1 1 1] Set Current Action
  (bind _output_get (Variables|Default|SetCurrentAction CurrentAction))
  (switch Utilities|FlowControl|Switch|SwitchonE_CurrentActions _output_get
    (:NewEnumerator3
      (Default|SetOccupied (Variables|Default|GetTargetSeat) false)
      (AI|Navigation|SimpleMovetoLocation (Pawn|GetController) (Variables|Default|GetSpawnLocation)))))

(event Custom|DelayPathfingToLetSomeoneStandUp
  (params (Delay :type Float%20%28single-precision%29))
  ;[1 1 1] Move To
  (AI|Navigation|StopMovement (Pawn|GetController))
  (Utilities|FlowControl|RetriggerableDelay Delay)
  (AI|AIMoveTo (AI|GetAIController self) self (Transformation|GetActorLocation (Variables|Default|GetTargetSeat)) 0 5.0 false
    (:OnSuccess
      (Variables|Default|SetCurrentAction "NewEnumerator1")
      (Default|SetOccupied (Variables|Default|GetTargetSeat) true)
      (AI|Navigation|StopMovement (Pawn|GetController)))))

(event Custom|PlayFacialMorphTarget
  (params (FacialAnim :type E_FacialAnimations%20Enum :default "NewEnumerator0"))
  ;[1 1 1] Facial Morph
  (bind _returnvalue (Utilities|GetDataTableRow "/Game/Blueprints/Audience/Face/DT_FacialAnimations.DT_FacialAnimations" (Utilities|String|StringToName (Utilities|String|EnumtoString FacialAnim)))
    (:then
      (bind _time (Timeline|FacialAnimation PlayFromStart)
        (:Update
          (for _array_element (Utilities|Struct|BreakS_FacialAnimations _returnvalue)
            (Components|SkeletalMesh|SetMorphTarget (Variables|Character|GetMesh) (.MorphTarget (Utilities|Struct|BreakS_FacialAnimation _array_element)) (Math|Curves|GetFloatValue (.Curve (Utilities|Struct|BreakS_FacialAnimation _array_element)) _time) true)))))))

(event EventTick
  (params (DeltaSeconds :type Float%20%28single-precision%29))
  (bind _returnvalue (Transformation|GetActorRotation))
  (bind _returnvalue_2 (Transformation|GetActorForwardVector))
  (bind _returnvalue_3 (Transformation|GetActorLocation))
  (bind _targetseat (Variables|Default|GetTargetSeat))
  (bind _currentaction (Variables|Default|GetCurrentAction))
  (bind _returnvalue_4 (Math|Vector|NegateVector _returnvalue_2))
  (bind _returnvalue_5 (Transformation|GetActorLocation _targetseat))
  (bind _returnvalue_6 (Utilities|Enum|Equal(Enum) _currentaction "NewEnumerator1"))
  (bind _returnvalue_7 (* _returnvalue_4 5e+01))
  (bind _returnvalue_8 (Math|Interpolation|VInterpTo _returnvalue_3 _returnvalue_5 DeltaSeconds 5.0))
  (bind _returnvalue_9 (+ _returnvalue_7 _returnvalue_5))
  (bind _returnvalue_10 (Math|Interpolation|VInterpTo _returnvalue_3 _returnvalue_9 DeltaSeconds 5.0))
  (bind _returnvalue_11 (select _returnvalue_6 _returnvalue_8 _returnvalue_10))
  ;[1 1 1] Tick Current Action
  (Utilities|IsValid (Variables|Default|GetTargetSeat)
    (:Is%20Valid
      (switch Utilities|FlowControl|Switch|SwitchonE_CurrentActions (Variables|Default|GetCurrentAction)
        (:NewEnumerator1
          ;[1 1 1] Rotate
          (Transformation|SetActorRotation (Math|Rotator|MakeRotator (.roll _returnvalue) (.pitch _returnvalue) (Math|Interpolation|FInterpTo (.yaw _returnvalue) (Class|KismetMathLibrary|ClampAxis (+ (.yaw (Transformation|GetWorldRotation (Variables|/Game/Blueprints/BP_Seat.BP_Seat_C|GetSM_Seat (Variables|Default|GetTargetSeat)))) 1.8e+02)) DeltaSeconds 5.0)))
          ;[1 1 1] Facial
          (if (== (Math|Random|RandomInteger 500) 0)
            (CallFunction|PlayFacialMorphTarget "NewEnumerator0")))
        (:NewEnumerator2
          _))
      ;[1 1 1] Shift to Let someone through
      (Transformation|SetActorLocation (Math|Vector|MakeVector (.x _returnvalue_11) (.y _returnvalue_11) (.z (Transformation|GetActorLocation))) false false))))

(event EventBeginPlay
  ;[1 1 1] Spawn Location
  (Variables|Default|SetSpawnLocation (Transformation|GetActorLocation))
  (CallFunction|GenerateAppearance))

(fn ConstructionScript)

(fn GenerateAppearance
  (bind _mesh (Variables|Character|GetMesh))
  (bind _mesh_2 (Variables|Character|GetMesh))
  ;[1 1 1] Choose Random Appearance
  (bind _appearances (CallFunction|GetMatchingAppearances))
  (bind _output_get (LocalVariables|SetChosenAppearance (Utilities|Array|Get(acopy) _appearances (Math|Random|RandomInteger (Utilities|Array|Length _appearances)))))
  ;[1 1 1] Apply Stuff to SM
  (Components|SkeletalMesh|SetAnimInstanceClass _mesh_2 (.AnimationBP (Utilities|Struct|BreakS_AppearanceInfo _output_get)))
  (Class|SkinnedMeshComponent|SetSkeletalMesh _mesh_2 (.SkeletalMesh (Utilities|Struct|BreakS_AppearanceInfo _output_get)) true)
  (for _array_element (.MaterialSwitches (Utilities|Struct|BreakS_AppearanceInfo (LocalVariables|GetChosenAppearance)))
    (Rendering|Material|SetMaterial (Variables|Character|GetMesh) (.SlotID (Utilities|Struct|BreakS_MaterialSwitch _array_element)) (Utilities|Array|Get(acopy) (.Materials (Utilities|Struct|BreakS_MaterialSwitch _array_element)) (Math|Random|RandomInteger (Utilities|Array|Length (.Materials (Utilities|Struct|BreakS_MaterialSwitch _array_element)))))))
  (for _array_element_2 (.MaterialModifier (Utilities|Struct|BreakS_AppearanceInfo (LocalVariables|GetChosenAppearance)))
    (bind _returnvalue (Rendering|Material|CreateDynamicMaterialInstance _mesh (.MaterialID (Utilities|Struct|BreakS_MaterialModifier _array_element_2)) (Rendering|Material|GetMaterial _mesh (.MaterialID (Utilities|Struct|BreakS_MaterialModifier _array_element_2))) "None" :!class /Script/Engine.PrimitiveComponent))
    (Rendering|Material|SetVectorParameterValue _returnvalue (.ParameterName (Utilities|Struct|BreakS_MaterialModifier _array_element_2)) (Math|Conversions|ToLinearColor(Color) (Utilities|Array|Get(acopy) (.Colors (Utilities|Struct|BreakS_MaterialModifier _array_element_2)) (Math|Random|RandomInteger (Utilities|Array|Length (.Colors (Utilities|Struct|BreakS_MaterialModifier _array_element_2)))))) :!class /Script/Engine.MaterialInstanceDynamic))
  ;[1 1 1] Randomize Actor Scale Z
  (Transformation|SetActorScale3D (Math|Vector|MakeVector 1.0 1.0 (Math|Random|RandomFloatinRange 0.9 1.1))))

(fn GetMatchingAppearances
  (bind _outrownames (DataTable|GetDataTableRowNames "/Game/Blueprints/Audience/AppearanceGeneration/DT_Appearance.DT_Appearance"))
  (for _array_element _outrownames
    (bind _returnvalue (Utilities|GetDataTableRow "/Game/Blueprints/Audience/AppearanceGeneration/DT_Appearance.DT_Appearance" _array_element)
      (:then
        (if (and (Math|Boolean|Equal(Boolean) (.Male (Utilities|Struct|BreakS_AppearanceInfo _returnvalue)) (Variables|Default|GetIsMale)) (Math|Boolean|Equal(Boolean) (.Reputable (Utilities|Struct|BreakS_AppearanceInfo _returnvalue)) (Variables|Default|GetIsReputable)))
          (Utilities|Array|Add (Variables|Default|GetAppearance) _returnvalue)))))
  (return (Variables|Default|GetAppearance)))