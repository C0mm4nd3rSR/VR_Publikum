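; BP_SeatRow is an actor that builds a straight row of BP_Seat actors.
; The construction script adds a configurable number of child actor components, spaced along local X by a fixed offset.
; On BeginPlay it reads the root's direct child components and stores each spawned BP_Seat in a Seats array.
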(event EventBeginPlay
  ;[1 1 1] Add Seats
  (for _array_element (Components|GetChildrenComponents (Variables|Default|GetDefaultSceneRoot) false)
    (bind _aschild_actor_component (Utilities|Casting|CastToChildActorComponent _array_element))
    (bind _asbp_seat (Utilities|Casting|CastToBP_Seat (Variables|/Script/Engine.ChildActorComponent|GetChildActor _aschild_actor_component)))
    (Utilities|Array|Add (Variables|Default|GetSeats) _asbp_seat)))

(fn ConstructionScript
  (for _index (range 0 (- (Variables|Default|GetNUM_SEATS) 1))
    (bind _returnvalue (AddComponent|AddChildActorComponent false (Math|Transform|MakeTransform (Math|Vector|MakeVector (Math|Conversions|ToFloat(Integer) (* _index (Variables|Default|GetSPAWN_X_OFFSET))) 0.0 0.0) "0, 0, 0" "1,1,1")))
    (ChildActorComponent|SetChildActorClass _returnvalue "/Game/Blueprints/BP_Seat.BP_Seat_C")))